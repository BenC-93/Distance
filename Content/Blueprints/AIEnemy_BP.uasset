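; AI enemy Blueprint, apparently themed on loneliness, that adds trigger and sound hooks to enemy logic defined outside these graphs.
; Attack box overlaps log and forward the other actor to OnAttackTrigger or OnExitAttackTrigger, while range overlaps are empty.
; BPPlay events start audio only if not already playing, with the death event reusing the drain component.
; An explosion emitter and extra log calls are left unconnected.
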(event `self.AITriggerAttack.OnComponentBeginOverlap`
  (params (OtherActor :type "Actor Object Reference") (OtherComp :type "PrimitiveComponent Object Reference") (OtherBodyIndex :type Integer) (bFromSweep :type Boolean) (SweepResult :type "EngineTypes.HitResult Structure (by ref)"))
  (`VisualLoggerKismetLibrary.LogText` "OMG entered box")
  (`self.OnAttackTrigger` self OtherActor))

(event `self.AITriggerAttack.OnComponentEndOverlap`
  (params (OtherActor :type "Actor Object Reference") (OtherComp :type "PrimitiveComponent Object Reference") (OtherBodyIndex :type Integer))
  (`VisualLoggerKismetLibrary.LogText` "OMG exited trigger box")
  (`self.OnExitAttackTrigger` OtherActor))

(event `self.AITriggerRange.OnComponentBeginOverlap`
  (params (OtherActor :type "Actor Object Reference") (OtherComp :type "PrimitiveComponent Object Reference") (OtherBodyIndex :type Integer) (bFromSweep :type Boolean) (SweepResult :type "EngineTypes.HitResult Structure (by ref)")))

(event `self.BPPlayTriggerSound`
  (bind _lonelinessbeginaudiocomponent (`self.LonelinessBeginAudioComponent`))
  ;[1 1 1] SoundFX
  (bind _returnvalue (`AudioComponent.IsPlaying` _lonelinessbeginaudiocomponent))
  (if (not _returnvalue)
    (`AudioComponent.Play` _lonelinessbeginaudiocomponent 0.0)))

(event `self.BPPlayDrainSound`
  (bind _lonelinessdrainaudiocomponent (`self.LonelinessDrainAudioComponent`))
  ;[1 1 1] SoundFX
  (bind _returnvalue (`AudioComponent.IsPlaying` _lonelinessdrainaudiocomponent))
  (if (not _returnvalue)
    (`AudioComponent.Play` _lonelinessdrainaudiocomponent 0.0)))

(event `self.BPPlayDeathSound`
  (bind _lonelinessdrainaudiocomponent (`self.LonelinessDrainAudioComponent`))
  ;[1 1 1] SoundFX
  (bind _returnvalue (`AudioComponent.IsPlaying` _lonelinessdrainaudiocomponent))
  (if (not _returnvalue)
    (`AudioComponent.Play` _lonelinessdrainaudiocomponent 0.0)))

(event `self.AITriggerRange.OnComponentEndOverlap`
  (params (OtherActor :type "Actor Object Reference") (OtherComp :type "PrimitiveComponent Object Reference") (OtherBodyIndex :type Integer)))

(fn `UserConstructionScript`)